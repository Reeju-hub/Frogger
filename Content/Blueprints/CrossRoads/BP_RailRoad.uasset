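; Railroad lane for a Crossroads-style game that randomly sends trains and extends the level.
; A delayed Tick rolls about once a second to spawn BP_Train, play the alarm and flash the lights; a non-looping MultiGate plays each pass sound once.
; Player overlaps with walls and boxes nudge the chicken back every tick.
; Other triggers spawn the next land once through RailroadSpawner and clear the player's IsOnWater flag.
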(event OnComponentBeginOverlap(TriggerZone)
  (params (OverlappedComponent :type Primitive%20Component%20Object%20Reference) (OtherActor :type Actor%20Object%20Reference) (OtherComp :type Primitive%20Component%20Object%20Reference) (OtherBodyIndex :type Integer) (bFromSweep :type Boolean) (SweepResult :type Hit%20Result%20Structure%20%28by%20ref%29))
  (if (not (Variables|Default|GetRailroadSpawned))
    (Utilities|Casting|CastToBP_Player OtherActor)
    (Utilities|IsValid (Variables|Default|GetRailroadSpawner)
      (:Is%20Valid
        (Default|SpawnLandatSpawnPoint (Variables|Default|GetRailroadSpawner))
        (Variables|Default|SetRailroadSpawned true)))))

(event OnComponentBeginOverlap(DetectChicken)
  (params (OverlappedComponent :type Primitive%20Component%20Object%20Reference) (OtherActor :type Actor%20Object%20Reference) (OtherComp :type Primitive%20Component%20Object%20Reference) (OtherBodyIndex :type Integer) (bFromSweep :type Boolean) (SweepResult :type Hit%20Result%20Structure%20%28by%20ref%29))
  (bind _asbp_player (Utilities|Casting|CastToBP_Player OtherActor))
  (Variables|/Game/Blueprints/CrossRoads/BP_Player.BP_Player_C|SetIsOnWater _asbp_player false))

(event OnComponentBeginOverlap(Box2)
  (params (OverlappedComponent :type Primitive%20Component%20Object%20Reference) (OtherActor :type Actor%20Object%20Reference) (OtherComp :type Primitive%20Component%20Object%20Reference) (OtherBodyIndex :type Integer) (bFromSweep :type Boolean) (SweepResult :type Hit%20Result%20Structure%20%28by%20ref%29))
  (Utilities|Casting|CastToBP_Player OtherActor)
  (Variables|Default|SetOverlapped true))

(event OnComponentEndOverlap(Box2)
  (params (OverlappedComponent :type Primitive%20Component%20Object%20Reference) (OtherActor :type Actor%20Object%20Reference) (OtherComp :type Primitive%20Component%20Object%20Reference) (OtherBodyIndex :type Integer))
  (Utilities|Casting|CastToBP_Player OtherActor)
  (Variables|Default|SetOverlapped false))

(event OnComponentBeginOverlap(Wall1)
  (params (OverlappedComponent :type Primitive%20Component%20Object%20Reference) (OtherActor :type Actor%20Object%20Reference) (OtherComp :type Primitive%20Component%20Object%20Reference) (OtherBodyIndex :type Integer) (bFromSweep :type Boolean) (SweepResult :type Hit%20Result%20Structure%20%28by%20ref%29))
  (Utilities|Casting|CastToBP_Player OtherActor)
  (Variables|Default|SetOverlapped true))

(event OnComponentEndOverlap(Wall1)
  (params (OverlappedComponent :type Primitive%20Component%20Object%20Reference) (OtherActor :type Actor%20Object%20Reference) (OtherComp :type Primitive%20Component%20Object%20Reference) (OtherBodyIndex :type Integer))
  (Utilities|Casting|CastToBP_Player OtherActor)
  (Variables|Default|SetOverlapped false))

(event OnComponentBeginOverlap(Wall2)
  (params (OverlappedComponent :type Primitive%20Component%20Object%20Reference) (OtherActor :type Actor%20Object%20Reference) (OtherComp :type Primitive%20Component%20Object%20Reference) (OtherBodyIndex :type Integer) (bFromSweep :type Boolean) (SweepResult :type Hit%20Result%20Structure%20%28by%20ref%29))
  (Utilities|Casting|CastToBP_Player OtherActor)
  (Variables|Default|SetOverlapped true))

(event OnComponentEndOverlap(Wall2)
  (params (OverlappedComponent :type Primitive%20Component%20Object%20Reference) (OtherActor :type Actor%20Object%20Reference) (OtherComp :type Primitive%20Component%20Object%20Reference) (OtherBodyIndex :type Integer))
  (Utilities|Casting|CastToBP_Player OtherActor)
  (Variables|Default|SetOverlapped false))

(event OnComponentBeginOverlap(RailLightBox)
  (params (OverlappedComponent :type Primitive%20Component%20Object%20Reference) (OtherActor :type Actor%20Object%20Reference) (OtherComp :type Primitive%20Component%20Object%20Reference) (OtherBodyIndex :type Integer) (bFromSweep :type Boolean) (SweepResult :type Hit%20Result%20Structure%20%28by%20ref%29))
  (Utilities|Casting|CastToBP_Player OtherActor)
  (Variables|Default|SetOverlapped true))

(event OnComponentEndOverlap(RailLightBox)
  (params (OverlappedComponent :type Primitive%20Component%20Object%20Reference) (OtherActor :type Actor%20Object%20Reference) (OtherComp :type Primitive%20Component%20Object%20Reference) (OtherBodyIndex :type Integer))
  (Utilities|Casting|CastToBP_Player OtherActor)
  (Variables|Default|SetOverlapped false))

(event OnComponentBeginOverlap(Box1)
  (params (OverlappedComponent :type Primitive%20Component%20Object%20Reference) (OtherActor :type Actor%20Object%20Reference) (OtherComp :type Primitive%20Component%20Object%20Reference) (OtherBodyIndex :type Integer) (bFromSweep :type Boolean) (SweepResult :type Hit%20Result%20Structure%20%28by%20ref%29))
  (Utilities|Casting|CastToBP_Player OtherActor)
  (Variables|Default|SetOverlapped true))

(event OnComponentEndOverlap(Box1)
  (params (OverlappedComponent :type Primitive%20Component%20Object%20Reference) (OtherActor :type Actor%20Object%20Reference) (OtherComp :type Primitive%20Component%20Object%20Reference) (OtherBodyIndex :type Integer))
  (Utilities|Casting|CastToBP_Player OtherActor)
  (Variables|Default|SetOverlapped false))

(event EventBeginPlay)

(event EventTick
  (params (DeltaSeconds :type Float%20%28single-precision%29))
  (Utilities|FlowControl|Sequence
    (:then_0
      (Utilities|FlowControl|Delay 1.0)
      (if (== (Math|Random|RandomInteger 20) 0)
        (CallFunction|SpawnTrain)
        (bind _asbp_player (Utilities|Casting|CastToBP_Player (Game|GetPlayerCharacter 0)))
        (Audio|SpawnSoundatLocation "/Game/Sounds/Train_Alarm_Cue.Train_Alarm_Cue" (Transformation|GetWorldLocation (Variables|/Game/Blueprints/CrossRoads/BP_Player.BP_Player_C|GetRotateChicken _asbp_player)) "0, 0, 0" 1.0 1.0 0.0 0 0)
        (Rendering|Material|SetMaterial (Variables|Default|GetLight2) 0 "/Game/Textures/largecar_mat1_2.largecar_mat1_2")
        (Rendering|Material|SetMaterial (Variables|Default|GetLight1) 0 "/Game/Textures/largecar_mat1_2.largecar_mat1_2")
        (Utilities|FlowControl|Delay 0.5)
        (Rendering|Material|SetMaterial (Variables|Default|GetLight2) 0 "/Game/Textures/Material_001.Material_001")
        (Rendering|Material|SetMaterial (Variables|Default|GetLight1) 0 "/Game/Textures/Material_001.Material_001")
        (Utilities|FlowControl|MultiGate true false -1
          (:Out%200
            (Audio|PlaySoundatLocation "/Game/Sounds/train_pass_shorter_Cue.train_pass_shorter_Cue" (Transformation|GetWorldLocation (Variables|/Game/Blueprints/CrossRoads/BP_Player.BP_Player_C|GetRotateChicken _asbp_player)) "0, 0, 0" 1.0 1.0 0.0 0 0 0 0))
          (:Out%201
            (Audio|PlaySoundatLocation "/Game/Sounds/train_pass_no_horn_Cue.train_pass_no_horn_Cue" (Transformation|GetWorldLocation (Variables|/Game/Blueprints/CrossRoads/BP_Player.BP_Player_C|GetRotateChicken _asbp_player)) "0, 0, 0" 1.0 1.0 0.0 0 0 0 0)))))
    (:then_1
      (if (Variables|Default|GetOverlapped)
        (bind _asbp_player_2 (Utilities|Casting|CastToBP_Player (Game|GetPlayerCharacter 0)))
        (Transformation|AddLocalOffset (Variables|/Game/Blueprints/CrossRoads/BP_Player.BP_Player_C|GetRotateChicken _asbp_player_2) "-15.000000, 0, 0" false false)))))

(fn ConstructionScript)

(fn SpawnTrain
  (bind _returnvalue (Game|SpawnActorfromClass "/Game/Blueprints/CrossRoads/BP_Train.BP_Train_C" (Math|Transform|MakeTransform (Transformation|GetWorldLocation (Variables|Default|GetTrainSpawn)) "0, 0, 0" "1.000000,1.000000,1.000000") "Undefined" "MultiplyWithRoot" 0 0))
  (Variables|/Game/Blueprints/CrossRoads/BP_Train.BP_Train_C|SetRailroadRef _returnvalue self))