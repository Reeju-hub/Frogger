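; MediumTree is a tree obstacle that blocks the player's chicken in what appears to be a road-crossing game.
; Box overlap events with BP_Player set a flag, and while it is set Tick pushes the player's RotateChicken component backward along local X by a fixed, unswept step per frame.
; Tick also polls the player's Restarting flag and destroys the MediumTree component once, leaving the actor itself alive.
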(event OnComponentBeginOverlap(Box)
  (params (OverlappedComponent :type Primitive%20Component%20Object%20Reference) (OtherActor :type Actor%20Object%20Reference) (OtherComp :type Primitive%20Component%20Object%20Reference) (OtherBodyIndex :type Integer) (bFromSweep :type Boolean) (SweepResult :type Hit%20Result%20Structure%20%28by%20ref%29))
  (Utilities|Casting|CastToBP_Player OtherActor)
  (Variables|Default|SetOverlapped true))

(event OnComponentEndOverlap(Box)
  (params (OverlappedComponent :type Primitive%20Component%20Object%20Reference) (OtherActor :type Actor%20Object%20Reference) (OtherComp :type Primitive%20Component%20Object%20Reference) (OtherBodyIndex :type Integer))
  (Utilities|Casting|CastToBP_Player OtherActor)
  (Variables|Default|SetOverlapped false))

(event EventBeginPlay)

(event EventTick
  (params (DeltaSeconds :type Float%20%28single-precision%29))
  (Utilities|FlowControl|Sequence
    (:then_0
      (if (not (Variables|Default|GetTreeDestroyed))
        (bind _asbp_player (Utilities|Casting|CastToBP_Player (Game|GetPlayerCharacter 0)))
        (if (Variables|/Game/Blueprints/CrossRoads/BP_Player.BP_Player_C|GetRestarting _asbp_player)
          (Components|DestroyComponent (Variables|Default|GetMediumTree))
          (Variables|Default|SetTreeDestroyed true))))
    (:then_1
      (if (Variables|Default|GetOverlapped)
        (bind _asbp_player_2 (Utilities|Casting|CastToBP_Player (Game|GetPlayerCharacter 0)))
        (Transformation|AddLocalOffset (Variables|/Game/Blueprints/CrossRoads/BP_Player.BP_Player_C|GetRotateChicken _asbp_player_2) "-15.000000, 0, 0" false false)))))

(fn ConstructionScript)