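; Road tile for a Crossy Road-style chicken game that spawns traffic and has RoadSpawner add the next land piece when the player first enters its trigger.
; BeginPlay randomly picks a spawn side and Speed via MultiGates.
; A Delay on Tick paces random car or truck spawns, which receive a road reference, plus engine or horn sounds at the player.
; Side walls nudge the overlapping chicken backward, and another overlap clears its water flag.
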(event OnComponentBeginOverlap(TriggerZone)
  (params (OverlappedComponent :type Primitive%20Component%20Object%20Reference) (OtherActor :type Actor%20Object%20Reference) (OtherComp :type Primitive%20Component%20Object%20Reference) (OtherBodyIndex :type Integer) (bFromSweep :type Boolean) (SweepResult :type Hit%20Result%20Structure%20%28by%20ref%29))
  (if (not (Variables|Default|GetRoadSpawned))
    (Utilities|Casting|CastToBP_Player OtherActor)
    (Utilities|IsValid (Variables|Default|GetRoadSpawner)
      (:Is%20Valid
        (Default|SpawnLandatSpawnPoint (Variables|Default|GetRoadSpawner))
        (Variables|Default|SetRoadSpawned true)))))

(event OnComponentBeginOverlap(DetectChicken)
  (params (OverlappedComponent :type Primitive%20Component%20Object%20Reference) (OtherActor :type Actor%20Object%20Reference) (OtherComp :type Primitive%20Component%20Object%20Reference) (OtherBodyIndex :type Integer) (bFromSweep :type Boolean) (SweepResult :type Hit%20Result%20Structure%20%28by%20ref%29))
  (bind _asbp_player (Utilities|Casting|CastToBP_Player OtherActor))
  (Variables|/Game/Blueprints/CrossRoads/BP_Player.BP_Player_C|SetIsOnWater _asbp_player false))

(event OnComponentBeginOverlap(Wall1)
  (params (OverlappedComponent :type Primitive%20Component%20Object%20Reference) (OtherActor :type Actor%20Object%20Reference) (OtherComp :type Primitive%20Component%20Object%20Reference) (OtherBodyIndex :type Integer) (bFromSweep :type Boolean) (SweepResult :type Hit%20Result%20Structure%20%28by%20ref%29))
  (Utilities|Casting|CastToBP_Player OtherActor)
  (Variables|Default|SetOverlapped true))

(event OnComponentEndOverlap(Wall1)
  (params (OverlappedComponent :type Primitive%20Component%20Object%20Reference) (OtherActor :type Actor%20Object%20Reference) (OtherComp :type Primitive%20Component%20Object%20Reference) (OtherBodyIndex :type Integer))
  (Utilities|Casting|CastToBP_Player OtherActor)
  (Variables|Default|SetOverlapped false))

(event OnComponentBeginOverlap(Wall2)
  (params (OverlappedComponent :type Primitive%20Component%20Object%20Reference) (OtherActor :type Actor%20Object%20Reference) (OtherComp :type Primitive%20Component%20Object%20Reference) (OtherBodyIndex :type Integer) (bFromSweep :type Boolean) (SweepResult :type Hit%20Result%20Structure%20%28by%20ref%29))
  (Utilities|Casting|CastToBP_Player OtherActor)
  (Variables|Default|SetOverlapped true))

(event OnComponentEndOverlap(Wall2)
  (params (OverlappedComponent :type Primitive%20Component%20Object%20Reference) (OtherActor :type Actor%20Object%20Reference) (OtherComp :type Primitive%20Component%20Object%20Reference) (OtherBodyIndex :type Integer))
  (Utilities|Casting|CastToBP_Player OtherActor)
  (Variables|Default|SetOverlapped false))

(event EventBeginPlay
  (Utilities|FlowControl|MultiGate true false -1
    (:Out%200
      (Variables|Default|SetSpawn1 true))
    (:Out%201
      (Variables|Default|SetSpawn2 true)))
  (Utilities|FlowControl|MultiGate true false -1
    (:Out%200
      (Variables|Default|SetSpeed "0,4.000000, 0"))
    (:Out%201
      (Variables|Default|SetSpeed "0,6.000000, 0"))
    (:Out%202
      (Variables|Default|SetSpeed "0,7.000000, 0"))))

(event Collision|EventActorBeginOverlap
  (params (OtherActor :type Actor%20Object%20Reference)))

(event EventTick
  (params (DeltaSeconds :type Float%20%28single-precision%29))
  (bind _returnvalue (Math|Random|RandomInteger 4))
  (Utilities|FlowControl|Sequence
    (:then_0
      (if (Variables|Default|GetOverlapped)
        (bind _asbp_player (Utilities|Casting|CastToBP_Player (Game|GetPlayerCharacter 0)))
        (Transformation|AddLocalOffset (Variables|/Game/Blueprints/CrossRoads/BP_Player.BP_Player_C|GetRotateChicken _asbp_player) "-15.000000, 0, 0" false false)))
    (:then_1
      (Utilities|FlowControl|Delay 1.0)
      (if (== _returnvalue 0)
        (CallFunction|SpawnLargeCar :!label _label)
        (if (not (Variables|Default|GetSoundPlaying)) :!label _label_2
          (Utilities|FlowControl|Delay 2.0)
          (Utilities|FlowControl|MultiGate true false -1
            (:Out%200
              (bind _asbp_player_2 (Utilities|Casting|CastToBP_Player (Game|GetPlayerCharacter 0)))
              (bind _returnvalue_2 (Audio|SpawnSoundatLocation "/Game/Sounds/car-engine-loop-deep_Cue.car-engine-loop-deep_Cue" (Transformation|GetWorldLocation (Variables|/Game/Blueprints/CrossRoads/BP_Player.BP_Player_C|GetRotateChicken _asbp_player_2)) "0, 0, 0" 1.0 1.0 0.0 0 0))
              (Variables|Default|SetSoundPlaying (Audio|Components|Audio|IsPlaying _returnvalue_2)))
            (:Out%201
              (bind _asbp_player_3 (Utilities|Casting|CastToBP_Player (Game|GetPlayerCharacter 0)))
              (bind _returnvalue_3 (Audio|SpawnSoundatLocation "/Game/Sounds/car-horn_Cue.car-horn_Cue" (Transformation|GetWorldLocation (Variables|/Game/Blueprints/CrossRoads/BP_Player.BP_Player_C|GetRotateChicken _asbp_player_3)) "0, 0, 0" 1.0 1.0 0.0 0 0))
              (Variables|Default|SetSoundPlaying (Audio|Components|Audio|IsPlaying _returnvalue_3)))))
        (elif (== _returnvalue 1)
          (goto _label)
          (elif (== _returnvalue 2)
            (CallFunction|SpawnTruck)
            (goto _label_2)))))))

(fn ConstructionScript)

(fn SpawnLargeCar
  (if (Variables|Default|GetSpawn1)
    (bind _returnvalue (Game|SpawnActorfromClass "/Game/Blueprints/CrossRoads/BP_LargeCar.BP_LargeCar_C" (Math|Transform|MakeTransform (Transformation|GetWorldLocation (Variables|Default|GetLargeCarSpawn1)) "0, 0, 0" "1.000000,1.000000,1.000000") "Undefined" "MultiplyWithRoot" 0 0))
    (Variables|/Game/Blueprints/CrossRoads/BP_LargeCar.BP_LargeCar_C|SetRoadRef _returnvalue self)
    (elif (Variables|Default|GetSpawn2)
      (bind _returnvalue_2 (Game|SpawnActorfromClass "/Game/Blueprints/CrossRoads/BP_LargeCar.BP_LargeCar_C" (Math|Transform|MakeTransform (Transformation|GetWorldLocation (Variables|Default|GetLargeCarSpawn2)) "0, 0, 0" "1.000000,1.000000,1.000000") "Undefined" "MultiplyWithRoot" 0 0))
      (Variables|/Game/Blueprints/CrossRoads/BP_LargeCar.BP_LargeCar_C|SetRoadRef _returnvalue_2 self))))

(fn SpawnTruck
  (if (Variables|Default|GetSpawn1)
    (bind _returnvalue (Game|SpawnActorfromClass "/Game/Blueprints/CrossRoads/BP_Truck.BP_Truck_C" (Math|Transform|MakeTransform (Transformation|GetWorldLocation (Variables|Default|GetTruckSpawn1)) "0, 0, 0" "1.000000,1.000000,1.000000") "Undefined" "MultiplyWithRoot" 0 0))
    (Variables|/Game/Blueprints/CrossRoads/BP_Truck.BP_Truck_C|SetRoadRef _returnvalue self)
    (elif (Variables|Default|GetSpawn2)
      (bind _returnvalue_2 (Game|SpawnActorfromClass "/Game/Blueprints/CrossRoads/BP_Truck.BP_Truck_C" (Math|Transform|MakeTransform (Transformation|GetWorldLocation (Variables|Default|GetTruckSpawn2)) "0, 0, 0" "1.000000,1.000000,1.000000") "Undefined" "MultiplyWithRoot" 0 0))
      (Variables|/Game/Blueprints/CrossRoads/BP_Truck.BP_Truck_C|SetRoadRef _returnvalue_2 self))))