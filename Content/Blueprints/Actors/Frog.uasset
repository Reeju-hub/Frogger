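; Frog Blueprint that turns move input into hopping movement for the player character.
; IA_Move input past a dead zone launches player 0's character upward and along world X for forward/backward or world Y for right/left.
; Each hop calls MovementCoolDown, which uses a DoOnce and a delay to block CanMove for two seconds before the next jump.
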(event Custom|MovementCoolDown
  ;[0.05729 0.05729 0.05729] WaitForNextJump
  (Utilities|FlowControl|DoOnce false :!label _label
    (:Completed
      (Variables|Default|SetCanMove false)
      (Utilities|FlowControl|Delay 2.0)
      (Variables|Default|SetCanMove true)
      (goto _label Reset))))

(event Input|EnhancedActionEvents|EnhancedInputActionIA_Move
  (params (ActionValue :type Vector%202D%20Structure) (ElapsedSeconds :type Float%20%28double-precision%29) (TriggeredSeconds :type Float%20%28double-precision%29) (InputAction :type Input%20Action%20Object%20Reference :default "/Game/ThirdPerson/Input/Actions/IA_Move.IA_Move"))
  ;[0.04688 0.04688 0.04688] Right/Left Movement
  (:Triggered
    (if (and (> (Math|Float|Absolute(Float) (.x ActionValue)) 0.3) (Variables|Default|GetCanMove))
      (CallFunction|MovementCoolDown)
      (Character|LaunchCharacter (Game|GetPlayerCharacter 0) (Math|Vector|MakeVector 0.0 (* (.x ActionValue) 3e+02) 1e+03) true true))))

(event Input|EnhancedActionEvents|EnhancedInputActionIA_Move
  (params (ActionValue :type Vector%202D%20Structure) (ElapsedSeconds :type Float%20%28double-precision%29) (TriggeredSeconds :type Float%20%28double-precision%29) (InputAction :type Input%20Action%20Object%20Reference :default "/Game/ThirdPerson/Input/Actions/IA_Move.IA_Move"))
  ;[0.0625 0.0625 0.0625] Forward/Backward Movement
  (:Triggered
    (if (and (> (Math|Float|Absolute(Float) (.y ActionValue)) 0.3) (Variables|Default|GetCanMove))
      (CallFunction|MovementCoolDown)
      (Character|LaunchCharacter (Game|GetPlayerCharacter 0) (Math|Vector|MakeVector (* (.y ActionValue) 3e+02) 0.0 1e+03) true true))))

(event EventBeginPlay)

(event Collision|EventActorBeginOverlap
  (params (OtherActor :type Actor%20Object%20Reference)))

(event EventTick
  (params (DeltaSeconds :type Float%20%28single-precision%29)))

(fn ConstructionScript)