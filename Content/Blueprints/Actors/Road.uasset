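; Road lane actor that sends vehicles across itself and awards score when the frog lands on it.
; On BeginPlay it caches the Start and End locations, randomly fixes one as the spawn side, and starts a looping timer with a randomized interval.
; Each tick of that timer has a coin-flip chance to spawn a Vehicle rotated for that side.
; A DoOnce on the Road hit event limits the Frog0 score update to once.
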(event OnComponentHit(Road)
  (params (HitComponent :type Primitive%20Component%20Object%20Reference) (OtherActor :type Actor%20Object%20Reference) (OtherComp :type Primitive%20Component%20Object%20Reference) (NormalImpulse :type Vector :default "0, 0, 0") (Hit :type Hit%20Result%20Structure%20%28by%20ref%29))
  (bind _asfrog_0 (Utilities|Casting|CastToFrog0 OtherActor))
  (Utilities|FlowControl|DoOnce false
    (:Completed
      (Default|UpdateScore _asfrog_0))))

(event Custom|Spawn%20Vehicles
  (if (Math|Random|RandomBool)
    (if (Variables|Default|GetStartingCarLocation)
      (Game|SpawnActorfromClass "/Game/Blueprints/Actors/Vehicle.Vehicle_C" (Math|Transform|MakeTransform (Variables|Default|GetStartLocation) "0.000000,90.000000,0.000000" "1.000000,1.000000,1.000000") "Undefined" "MultiplyWithRoot" 0 0)
      (else
        (Game|SpawnActorfromClass "/Game/Blueprints/Actors/Vehicle.Vehicle_C" (Math|Transform|MakeTransform (Variables|Default|GetEndLocation) "0.000000,-90.000000,0.000000" "1.000000,1.000000,1.000000") "Undefined" "MultiplyWithRoot" 0 0)))))

(event EventBeginPlay
  (Variables|Default|SetStartLocation (Transformation|GetWorldLocation (Variables|Default|GetStart)))
  (Variables|Default|SetEndLocation (Transformation|GetWorldLocation (Variables|Default|GetEnd)))
  (Variables|Default|SetStartingCarLocation (Math|Random|RandomBool))
  (Utilities|Time|SetTimerbyEvent (delegate Custom|Spawn%20Vehicles) (Math|Random|RandomFloatinRange 2.0 3.0) true))

(fn ConstructionScript)