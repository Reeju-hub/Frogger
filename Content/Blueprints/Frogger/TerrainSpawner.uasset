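; Frogger terrain spawner that builds a 31-strip lane of terrain along X when play begins.
; The first strips are always grass; the rest randomly pick grass, road or water, with grass weighted double.
; A fixed grass strip partway along also gets a MoreCollision trigger.
; When Frog0 first overlaps that trigger, a DoOnce spawns another TerrainSpawner 31000 units further along X, chaining the terrain generation.
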(event Custom|OnActorBeginOverlap_Event
  (params (OverlappedActor :type Actor%20Object%20Reference) (OtherActor :type Actor%20Object%20Reference))
  (bind _terrainspawner (Variables|Default|GetTerrainSpawner))
  (bind _returnvalue (Transformation|GetWorldLocation _terrainspawner))
  (Utilities|Casting|CastToFrog0 OtherActor)
  (Utilities|FlowControl|DoOnce false
    (:Completed
      (bind _output_get (Variables|Default|SetSpawnLocation (Math|Vector|MakeVector (+ (.x _returnvalue) 3.1e+04) (.y _returnvalue) (.z _returnvalue))))
      (Game|SpawnActorfromClass "TerrainSpawner_C" (Math|Transform|MakeTransform _output_get "0, 0, 0" "1.000000,1.000000,1.000000") "Undefined" "MultiplyWithRoot" 0 0))))

(event EventBeginPlay
  (bind _terrainspawner (Variables|Default|GetTerrainSpawner))
  (bind _returnvalue (Transformation|GetWorldLocation _terrainspawner))
  (for _index (range 0 30)
    (Variables|Default|SetSpawnLocation (Math|Vector|MakeVector (+ (* _index 91) (.x _returnvalue)) (.y _returnvalue) (.z _returnvalue)))
    (if (Math|Integer|InRange(Integer) _index 0 2)
      (Game|SpawnActorfromClass "/Game/Blueprints/Frogger/GrassTerrain.GrassTerrain_C" (Math|Transform|MakeTransform (Variables|Default|GetSpawnLocation) "0, 0, 0" "1.000000,1.000000,1.000000") "Undefined" "MultiplyWithRoot" 0 0)
      (elif (Math|Integer|InRange(Integer) _index 3 9)
        (switch int (Math|Random|RandomIntegerinRange 0 3) :!label _label
          (:0
            (Game|SpawnActorfromClass "/Game/Blueprints/Frogger/GrassTerrain.GrassTerrain_C" (Math|Transform|MakeTransform (Variables|Default|GetSpawnLocation) "0, 0, 0" "1.000000,1.000000,1.000000") "Undefined" "MultiplyWithRoot" 0 0))
          (:1
            (Game|SpawnActorfromClass "/Game/Blueprints/Frogger/GrassTerrain.GrassTerrain_C" (Math|Transform|MakeTransform (Variables|Default|GetSpawnLocation) "0, 0, 0" "1.000000,1.000000,1.000000") "Undefined" "MultiplyWithRoot" 0 0))
          (:2
            (Game|SpawnActorfromClass "/Game/Blueprints/Frogger/Road.Road_C" (Math|Transform|MakeTransform (Variables|Default|GetSpawnLocation) "0, 0, 0" "1.000000,1.000000,1.000000") "Undefined" "MultiplyWithRoot" 0 0))
          (:3
            (Game|SpawnActorfromClass "/Game/Blueprints/Frogger/Water.Water_C" (Math|Transform|MakeTransform (Variables|Default|GetSpawnLocation) "0, 0, 0" "1.000000,1.000000,1.000000") "Undefined" "MultiplyWithRoot" 0 0)))
        (elif (== _index 10)
          (Game|SpawnActorfromClass "/Game/Blueprints/Frogger/GrassTerrain.GrassTerrain_C" (Math|Transform|MakeTransform (Variables|Default|GetSpawnLocation) "0, 0, 0" "1.000000,1.000000,1.000000") "Undefined" "MultiplyWithRoot" 0 0)
          (bind _returnvalue_2 (Game|SpawnActorfromClass "/Game/Blueprints/Frogger/MoreCollision.MoreCollision_C" (Math|Transform|MakeTransform (Variables|Default|GetSpawnLocation) "0, 0, 0" "1.000000,1.000000,1.000000") "Undefined" "MultiplyWithRoot" 0 0))
          (EventDispatchers|AssignOnActorBeginOverlap _returnvalue_2 (delegate Custom|OnActorBeginOverlap_Event))
          (elif (Math|Integer|InRange(Integer) _index 10 30)
            (goto _label)))))))

(fn ConstructionScript)