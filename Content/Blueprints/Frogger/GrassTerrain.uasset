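; GrassTerrain is a Frogger-style grass strip that randomly scatters tree or rock obstacles when play begins.
; It steps along Y from the Start component in 180-unit intervals over the Start-to-End distance, spawning Treerockspawn at roughly one slot in five.
; A hit on the Grass component by Frog0 reaches a DoOnce with no follow-up, as the score update is disconnected.
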(event OnComponentHit(Grass)
  (params (HitComponent :type Primitive%20Component%20Object%20Reference) (OtherActor :type Actor%20Object%20Reference) (OtherComp :type Primitive%20Component%20Object%20Reference) (NormalImpulse :type Vector :default "0, 0, 0") (Hit :type Hit%20Result%20Structure%20%28by%20ref%29))
  (bind _asfrog_0 (Utilities|Casting|CastToFrog0 OtherActor))
  (Utilities|FlowControl|DoOnce false))

(event EventBeginPlay
  (Variables|Default|SetStartLocation (Transformation|GetWorldLocation (Variables|Default|GetStart)))
  (Variables|Default|SetEndLocation (Transformation|GetWorldLocation (Variables|Default|GetEnd)))
  (for _index (range 0 (Math|Float|Truncate (/ (Math|Vector|Distance(Vector) (Variables|Default|GetStartLocation) (Variables|Default|GetEndLocation)) 1.8e+02)))
    (if (> (Math|Random|RandomFloat) 0.8)
      (Game|SpawnActorfromClass "/Game/Blueprints/Frogger/Treerockspawn.Treerockspawn_C" (Math|Transform|MakeTransform (Math|Vector|MakeVector (.x (Variables|Default|GetStartLocation)) (+ (* _index 180) (.Y (Math|Vector|BreakVector (Variables|Default|GetStartLocation)))) (.z (Variables|Default|GetStartLocation))) "0, 0, 0" "1.000000,1.000000,1.000000") "Undefined" "MultiplyWithRoot" 0 0))))

(fn ConstructionScript)